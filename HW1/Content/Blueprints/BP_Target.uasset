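; BP_Target is a shootable target actor that counts toward completing a level.
; Hits from BP_FirstPersonProjectile reduce its Health by a fixed amount; at zero it increments the player character's TargetsHit and destroys itself.
; Once TargetsHit reaches the character's TotalTargets, it loads LevelThreeHazards2 from LevelTwo-Hazards1, or LevelOneMenu from any other level.
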(event Collision|EventHit
  (params (MyComp :type Primitive%20Component%20Object%20Reference) (Other :type Actor%20Object%20Reference) (OtherComp :type Primitive%20Component%20Object%20Reference) (bSelfMoved :type Boolean) (HitLocation :type Vector :default "0, 0, 0") (HitNormal :type Vector :default "0, 0, 0") (NormalImpulse :type Vector :default "0, 0, 0") (Hit :type Hit%20Result%20Structure%20%28by%20ref%29))
  (Utilities|Casting|CastToBP_FirstPersonProjectile Other)
  (Variables|Default|SetHealth (- (Variables|Default|GetHealth) 34))
  (if (<= (Variables|Default|GetHealth) 0)
    (bind _asbp_first_person_character (Utilities|Casting|CastToBP_FirstPersonCharacter (Game|GetPlayerCharacter 0)))
    (bind _output_get (Variables|/Game/FirstPerson/Blueprints/BP_FirstPersonCharacter.BP_FirstPersonCharacter_C|SetTargetsHit _asbp_first_person_character (+ (Variables|/Game/FirstPerson/Blueprints/BP_FirstPersonCharacter.BP_FirstPersonCharacter_C|GetTargetsHit _asbp_first_person_character) 1)))
    (Actor|DestroyActor)
    (if (>= _output_get (Variables|/Game/FirstPerson/Blueprints/BP_FirstPersonCharacter.BP_FirstPersonCharacter_C|GetTotalTargets _asbp_first_person_character))
      (bind _returnvalue (Game|GetCurrentLevelName true))
      (if (Utilities|Enum|Equal(Enum) _returnvalue "LevelTwo-Hazards1")
        (Game|OpenLevel(byObjectReference) "/Game/LevelThree-Hazards2.LevelThree-Hazards2")
        (else
          (Game|OpenLevel(byObjectReference) "/Game/LevelOne-Menu.LevelOne-Menu"))))))

(fn ConstructionScript)